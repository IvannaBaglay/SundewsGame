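; Game mode for the 2D game that sets up the player's UI and handles respawning.
; BeginPlay enables the mouse cursor with game-and-UI input, shows the fight HUD, and pre-creates hidden note, mail, failed and success widgets.
; The mail widget receives references to both result screens.
; RespawnPlayer spawns a new pawn of the player's class at an offset from its location, possesses it and calls its Respawn.
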(event Custom|RespawnPlayer
  (params (Player :type BP%20Player%20Object%20Reference))
  (bind _returnvalue (Game|SpawnActorfromClass (Utilities|GetClass Player) (Math|Conversions|ToTransform(Vector) (- (Transformation|GetActorLocation Player) (Variables|Default|GetSpawn%20Transform%20Shift))) "Undefined" 0 0))
  (Pawn|Possess (Game|GetPlayerController 0) _returnvalue)
  (Default|Respawn _returnvalue))

(event EventBeginPlay
  (bind _returnvalue (Game|GetPlayerController 0))
  (Variables|/Script/Engine.PlayerController|SetbShowMouseCursor _returnvalue true)
  (Input|SetInputModeGameandUI _returnvalue 0 "DoNotLock" true false)
  (bind _returnvalue_2 (UserInterface|CreateWidget "/Game/UI/HUD/FightHUD/WBP_FightHUD.WBP_FightHUD_C"))
  (UserInterface|Viewport|AddtoViewport _returnvalue_2 0)
  (Variables|/Script/UMG.Widget|SetVisibility _returnvalue_2 "Visible")
  (bind _returnvalue_3 (UserInterface|CreateWidget "/Game/UI/NoteWidget/UI_ReadNoteWidget.UI_ReadNoteWidget_C"))
  (UserInterface|Viewport|AddtoViewport _returnvalue_3 0)
  (Widget|SetVisibility _returnvalue_3 "Hidden")
  (bind _returnvalue_4 (UserInterface|CreateWidget "/Game/UI/NoteWidget/UI_PersonaMail.UI_PersonaMail_C"))
  (Widget|SetVisibility _returnvalue_4 "Hidden")
  (bind _returnvalue_5 (UserInterface|CreateWidget "/Game/UI/UI_Failed.UI_Failed_C"))
  (Widget|SetVisibility _returnvalue_5 "Hidden")
  (Variables|/Game/UI/NoteWidget/UI_PersonaMail.UI_PersonaMail_C|SetFailedScreen _returnvalue_4 _returnvalue_5)
  (UserInterface|Viewport|AddtoViewport _returnvalue_5 0)
  (bind _returnvalue_6 (UserInterface|CreateWidget "/Game/UI/UI_Success.UI_Success_C"))
  (Variables|/Script/UMG.Widget|SetVisibility _returnvalue_6 "Hidden")
  (Variables|/Game/UI/NoteWidget/UI_PersonaMail.UI_PersonaMail_C|SetSuccessScreen _returnvalue_4 _returnvalue_6)
  (UserInterface|Viewport|AddtoViewport _returnvalue_6 0)
  (UserInterface|Viewport|AddtoViewport _returnvalue_4 0))

(event EventTick
  (params (DeltaSeconds :type Float%20%28single-precision%29)))

(fn ConstructionScript)