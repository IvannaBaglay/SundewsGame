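; Skeleton wisp enemy that fights the player in rounds of countering skill types, linked to a health bar in the fight HUD.
; Incoming damage picks a differing skill from AttackPattern, then CheckAbilitiesPower decides whether the skeleton takes damage or strikes back.
; Rounds update the HUD's used skills; death ends the fight and notifies its owning note actor.
; In the matchup check, player Shock always wins and the Wave branch is unreachable.
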(event OnComponentBeginOverlap(BoxAttack)
  (params (OverlappedComponent :type Primitive%20Component%20Object%20Reference) (OtherActor :type Actor%20Object%20Reference) (OtherComp :type Primitive%20Component%20Object%20Reference) (OtherBodyIndex :type Integer) (bFromSweep :type Boolean) (SweepResult :type Hit%20Result%20Structure%20%28by%20ref%29))
  ;[1 1 1] Begin Overlap attack box
  (Development|PrintString "Overlap box attack")
  (if (== OtherActor (Game|GetPlayerCharacter 0))
    (Variables|Default|SetAttackMode true)))

(event OnComponentEndOverlap(BoxAttack)
  (params (OverlappedComponent :type Primitive%20Component%20Object%20Reference) (OtherActor :type Actor%20Object%20Reference) (OtherComp :type Primitive%20Component%20Object%20Reference) (OtherBodyIndex :type Integer))
  ;[1 1 1] End Overlap attack box
  (if (== OtherActor (Game|GetPlayerCharacter 0))
    (Variables|Default|SetAttackMode false)
    (Utilities|Time|ClearandInvalidateTimerbyHandle (Variables|Default|GetAttackEvent))))

(event Custom|HandleRotation
  ;[1 1 1] Handle sprite direction
  (if (> (Variables|Default|GetMovementDirection) 0.0)
    (Transformation|SetActorRotation "0, 0, 0")
    (else
      (Transformation|SetActorRotation "0.000000,180.000000,0.000000"))))

(event Custom|EnemyAttacked
  (Class|PaperZDAnimInstance|JumptoNode (Variables|/Script/PaperZD.PaperZDAnimationComponent|GetAnimInstance (Variables|Default|GetAnimationComponent)) "Attack" "Enemy"))

(event Custom|Attack
  (bind _returnvalue (Transformation|GetActorLocation))
  (bind _returnvalue_2 (Game|GetPlayerCharacter 0))
  ;[1 1 1] Attack (can be deleted?)
  (bind _outhit (Collision|LineTraceForObjects _returnvalue (+ _returnvalue (* (Transformation|GetActorForwardVector) (Math|Vector|MakeVector 1e+02 0.0 0.0))) (Utilities|Array|MakeArray "ObjectTypeQuery3") false 0 "ForDuration"))
  (if (== (.HitActor (Collision|BreakHitResult _outhit)) _returnvalue_2)
    (Development|PrintString "Enemy damage Player" true true "(R=1.000000,G=0.018841,B=0.078564,A=1.000000)")
    (Game|Damage|ApplyDamage _returnvalue_2 1.0 0 0)))

(event Custom|StartFigth
  ;[1 1 1] Set up start fight
  (Development|PrintString "Start Fight Enemy" true true "(R=0.955831,G=0.000000,B=1.000000,A=1.000000)")
  (Variables|Default|SetAttackMode true))

(event EventBeginPlay
  ;[1 1 1] Begin Play
  (Variables|/Script/Engine.CharacterMovementComponent|SetMaxWalkSpeed (Variables|Character|GetCharacterMovement) (Variables|Default|GetMaxWalkSpeed))
  (Variables|Default|SetHealth (Variables|Default|GetMaxHealth))
  (bind _asbp_actor_note (Utilities|Casting|CastToBP_ActorNote (Components|GetOwner)))
  (Variables|Default|SetSpawnPoint _asbp_actor_note)
  (bind _foundwidgets (Widget|GetAllWidgetsOfClass "/Game/UI/HUD/FightHUD/WBP_FightHUD.WBP_FightHUD_C" true))
  (bind _output_get (Variables|Default|SetWBP%20Enemy%20Health%20Bar (Variables|/Game/UI/HUD/FightHUD/WBP_FightHUD.WBP_FightHUD_C|GetWBP_EnemyHealthBar (Utilities|Array|Get(acopy) _foundwidgets))))
  (Variables|/Game/UI/HUD/HealthHUD/WBP_EnemyHealthBar.WBP_EnemyHealthBar_C|SetSkeletonRef _output_get self)
  (Default|UpdateHealth _output_get))

(event Collision|EventActorBeginOverlap
  (params (OtherActor :type Actor%20Object%20Reference)))

(event Game|Damage|EventAnyDamage
  (params (Damage :type Float%20%28single-precision%29) (DamageType :type Damage%20Type%20Object%20Reference) (InstigatedBy :type Controller%20Object%20Reference) (DamageCauser :type Actor%20Object%20Reference))
  (bind _spawnpoint (Variables|Default|GetSpawnPoint))
  (bind _animationcomponent (Variables|Default|GetAnimationComponent))
  (bind _animinstance (Variables|/Script/PaperZD.PaperZDAnimationComponent|GetAnimInstance _animationcomponent))
  ;[1 1 1] Get Damage
  ;;[1 1 1] Get response attack and ckeck who win
  (Variables|Default|SetGetDamaged Damage)
  (Variables|Default|SetDamage%20Causer DamageCauser)
  (Variables|Default|SetCanHit true)
  (bind _choosendamagetype_ (CallFunction|ChooseContrAttack (Utilities|GetClass DamageType)))
  (Variables|Default|SetChoosen%20Damage%20Type _choosendamagetype_)
  (bind _playerwinshouldtakedamage (CallFunction|CheckAbilitiesPower (Utilities|GetClass DamageType) _choosendamagetype_))
  (Utilities|FlowControl|Sequence
    (:then_0
      (if _playerwinshouldtakedamage
        ;;[1 1 1] Get Damage
        (bind _output_get (Variables|Default|SetHealth (- (Variables|Default|GetHealth) (Variables|Default|GetGetDamaged))))
        (Default|EnemyDamaged (Variables|Default|GetWBP%20Enemy%20Health%20Bar))
        (if (<= _output_get 0.0)
          (Actor|DestroyActor)
          (Default|Clean (Variables|Default|GetWBP%20Enemy%20Health%20Bar))
          (Development|PrintString "Killed Skeleton" true true "(R=0.136170,G=0.189296,B=1.000000,A=1.000000)")
          (bind _asbp_player (Utilities|Casting|CastToBP_Player (Variables|Default|GetDamage%20Causer)))
          (Development|PrintString "Hello")
          (if (== _asbp_player (Game|GetPlayerCharacter 0))
            (Default|EndFight _asbp_player)
            (Utilities|IsValid _spawnpoint
              (:Is%20Valid
                (Default|ShowReadDelete _spawnpoint))))
          (else
            (Utilities|IsValid _animinstance
              (:Is%20Valid
                (Class|PaperZDAnimInstance|JumptoNode _animinstance "Damaged" "Enemy")
                (Development|PrintString "Damaged Skeleton" true true "(R=0.136170,G=0.189296,B=1.000000,A=1.000000)")
                (bind _asbp_player_2 (Utilities|Casting|CastToBP_Player (Game|GetPlayerCharacter 0)))
                (Default|NextStepActive _asbp_player_2)))))
        (else
          ;;[1 1 1] Apply damage if enemy win round
          (Game|Damage|ApplyDamage (Variables|Default|GetDamage%20Causer) 1.0 0 self _choosendamagetype_)
          (bind _asbp_player_3 (Utilities|Casting|CastToBP_Player (Game|GetPlayerCharacter 0)))
          (Default|NextStepActive _asbp_player_3))))
    (:then_1
      ;;[1 1 1] Update HUD Menu choosen skills
      (bind _foundwidgets (Widget|GetAllWidgetsOfClass "/Game/UI/HUD/FightHUD/WBP_FightHUD.WBP_FightHUD_C" true))
      (if (> (Utilities|Array|Length _foundwidgets) 0)
        (bind _asbp_damage_ty_general (Utilities|Casting|CastToBP_DamageTyGeneral DamageType))
        (bind _returnvalue (Game|ConstructObjectfromClass (Variables|Default|GetChoosen%20Damage%20Type)))
        (Default|UpdateUsedSkills (Utilities|Array|Get(acopy) _foundwidgets) (Variables|/Game/DamageTypes/BP_DamageTyGeneral.BP_DamageTyGeneral_C|GetName _returnvalue) (Variables|/Game/DamageTypes/BP_DamageTyGeneral.BP_DamageTyGeneral_C|GetName _asbp_damage_ty_general) (Variables|/Game/DamageTypes/BP_DamageTyGeneral.BP_DamageTyGeneral_C|GetImage _returnvalue) (Variables|/Game/DamageTypes/BP_DamageTyGeneral.BP_DamageTyGeneral_C|GetImage _asbp_damage_ty_general))))))

(fn ConstructionScript)

(fn ChooseContrAttack
  (params (DamageType :type Damage%20Type%20Class%20Reference))
  (bind _attackpattern (Variables|Default|GetAttackPattern))
  (bind _returnvalue (Utilities|Array|Length _attackpattern))
  (bind _index (Utilities|FlowControl|ForLoopwithBreak (Variables|Default|GetAttackIndex) (- _returnvalue 1) :!label _label)
    (:LoopBody
      (if (!= (Utilities|Array|Get(acopy) _attackpattern _index) DamageType)
        (if (>= (+ _index 1) _returnvalue)
          (Variables|Default|SetAttackIndex 0)
          (else
            (Variables|Default|SetAttackIndex (+ _index 1))
            (return (Utilities|Array|Get(acopy) _attackpattern _index))))))
    (:Completed
      (Variables|Default|SetAttackIndex 0)
      (goto _label))))

(fn CheckAbilitiesPower
  (params (PlayerDamage :type Damage%20Type%20Class%20Reference) (EnemyDamage :type Damage%20Type%20Class%20Reference))
  ;[1 1 1] If Player Attack Melee
  (if (== PlayerDamage "/Game/DamageTypes/BP_DamageType_Attack.BP_DamageType_Attack_C")
    (if (== EnemyDamage "/Game/DamageTypes/BP_DamageType_Shield.BP_DamageType_Shield_C")
      _
      (elif (== EnemyDamage "/Game/DamageTypes/BP_DamageType_Wave.BP_DamageType_Wave_C")
        _
        (else
          (return false))))
    (return true)
    (else
      ;[1 1 1] If Player Attack Shield
      (if (== PlayerDamage "/Game/DamageTypes/BP_DamageType_Shield.BP_DamageType_Shield_C")
        (if (== EnemyDamage "/Game/DamageTypes/BP_DamageType_Shock.BP_DamageType_Shock_C")
          _
          (elif (== EnemyDamage "/Game/DamageTypes/BP_DamageType_Shoot.BP_DamageType_Shoot_C")
            _
            (else
              (return false))))
        (return true)
        (else
          ;[1 1 1] If Player Attack Shock
          (if (== PlayerDamage "/Game/DamageTypes/BP_DamageType_Shock.BP_DamageType_Shock_C")
            (if (== EnemyDamage "/Game/DamageTypes/BP_DamageType_Shoot.BP_DamageType_Shoot_C")
              _
              (elif true
                _
                (else
                  (return false))))
            (return true)
            (else
              ;[1 1 1] If Player Attack Shoot
              (if (== PlayerDamage "/Game/DamageTypes/BP_DamageType_Shoot.BP_DamageType_Shoot_C")
                (if (== EnemyDamage "/Game/DamageTypes/BP_DamageType_Wave.BP_DamageType_Wave_C")
                  _
                  (elif (== EnemyDamage "/Game/DamageTypes/BP_DamageType_Attack.BP_DamageType_Attack_C")
                    _
                    (else
                      (return false))))
                (return true)))))))))